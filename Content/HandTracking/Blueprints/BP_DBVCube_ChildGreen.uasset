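; Green child variant of a hand-tracking cube that flashes when a VR hand touches it.
; Its mesh's begin-overlap event filters for BP_HandsVR, swaps material slot 0 to GlowMat, then after a 0.2-second delay sets that slot again with no material specified.
; The construction script only calls the parent, and the default BeginPlay, actor overlap and Tick events are disabled.
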(event `self.StaticMesh.OnComponentBeginOverlap`
  (params (OverlappedComponent :type "PrimitiveComponent Object Reference") (OtherActor :type "Actor Object Reference") (OtherComp :type "PrimitiveComponent Object Reference") (OtherBodyIndex :type Integer) (bFromSweep :type Boolean) (SweepResult :type "HitResult Structure (by ref)"))
  (cast `/Game/HandTracking/Blueprints/BP_HandsVR` OtherActor)
  (`PrimitiveComponent.SetMaterial` (`self.StaticMesh`) 0 (`self.GlowMat`))
  (`KismetSystemLibrary.Delay` 0.2)
  (`PrimitiveComponent.SetMaterial` (`self.StaticMesh`) 0 null))

(fn `UserConstructionScript`
  (`parent.UserConstructionScript`))