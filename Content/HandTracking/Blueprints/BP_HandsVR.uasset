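; BP_HandsVR is a Meta XR hands actor that sets up VR hand tracking and places in-world UI widgets.
; With an HMD active, BeginPlay sets local-floor tracking, Interaction SDK input mappings and animated controller hands, then moves "Start"-tagged widgets near the hand.
; The left menu input, gated on the hand's material being M_Hand1, shows the "Menu"-tagged widget by the hand or hides and moves it away.
; Restart reloads the current level.
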(event `self.ReceiveBeginPlay`
  (bind _returnvalue (pcsubsystem `EnhancedInputLocalPlayerSubsystem` (`GameplayStatics.GetPlayerController` 0)))
  ; Set Tracking Space
  (if (`HeadMountedDisplayFunctionLibrary.IsHeadMountedDisplayEnabled`)
    (`HeadMountedDisplayFunctionLibrary.SetTrackingOrigin` "LocalFloor")
    (`EnhancedInputSubsystemInterface.AddMappingContext` _returnvalue "/OculusInteraction/Inputs/IMC_IsdkHand.IMC_IsdkHand" 1 (struct))
    (`EnhancedInputSubsystemInterface.AddMappingContext` _returnvalue "/OculusInteraction/Inputs/IMC_IsdkControllerAnimation.IMC_IsdkControllerAnimation" 1 (struct))
    (`IsdkFunctionLibrary.SetControllerHandBehavior` "BothAnimated")
    (bind _outactors (`GameplayStatics.GetAllActorsOfClassWithTag` "/Script/OculusInteractionPrebuilts.IsdkInteractableWidget" "Start"))
    (for _array_element _outactors
      (`self.K2_SetActorLocation` _array_element (+ (`SceneComponent.K2_GetComponentLocation` (`self.OculusXRHand`)) (-45.0 0.0 100.0)) false false))))

(event `EnhancedInput|/Game/VRTemplate/Input/Actions/IA_Menu_Toggle_Left`
  (params (ActionValue :type Boolean) (ElapsedSeconds :type "Float (double-precision)") (TriggeredSeconds :type "Float (double-precision)") (InputAction :type "InputAction Object Reference" :default "/Game/VRTemplate/Input/Actions/IA_Menu_Toggle_Left.IA_Menu_Toggle_Left"))
  (bind (_returnvalue_roll _returnvalue_pitch _returnvalue_yaw) (`KismetMathLibrary.BreakRotator` (`SceneComponent.GetSocketRotation` (`self.LeftMotionController`) "None")))
  (:`Triggered`
    (if (and (== (`PrimitiveComponent.GetMaterial` (`self.OculusXRHand`) 0) "/Game/HandTracking/Blueprints/M_Hand1.M_Hand1") ActionValue)
      (bind _outactors (`GameplayStatics.GetAllActorsOfClassWithTag` "/Script/OculusInteractionPrebuilts.IsdkInteractableWidget" "Menu"))
      (bind _output (`|GetArrayItem` _outactors))
      (if (`Actor.bHidden` _output)
        (`self.SetActorHiddenInGame` _output false)
        (`self.K2_SetActorLocationAndRotation` _output (+ (`SceneComponent.K2_GetComponentLocation` (`self.OculusXRHand`)) (`self.Offset`)) (`KismetMathLibrary.MakeRotator` 0.0 _returnvalue_pitch (- _returnvalue_yaw 90.0)) false false)
        (else
          (`self.SetActorHiddenInGame` _output true)
          (`self.K2_SetActorLocation` _output (500.0 500.0 500.0) false true))))))

(fn `Restart`
  (bind _returnvalue (`GameplayStatics.GetCurrentLevelName` true))
  (`GameplayStatics.OpenLevel` (`KismetStringLibrary.Conv_StringToName` _returnvalue)))

(fn `UserConstructionScript`)