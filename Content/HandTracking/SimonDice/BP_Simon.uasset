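; Simon Says memory game actor for VR hand tracking, where the player repeats note sequences played on linked stands.
; Each level builds a random sequence from LevelSettings, plays it with timed delays and text prompts, then opens the player's turn.
; PlayerPlayedNote checks each note, advancing the level on completion or replaying the sequence on error.
; The construction script caps no-duplicate note counts to the stand count, and Tick keeps the actor offset from the VR camera.
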(event `CreateSimonSequence`
  (bind _previoussecuence (`self.PreviousSecuence`))
  (bind _simonsequence (`self.SimonSequence`))
  (bind ((`NumberOfNotes_2_B7FEC37945633957BFED269576B25116` _numberofnotes) (`CanDuplicateNotes_8_50756D694749D8014C6791A38BD63140` _canduplicatenotes)) (break `/Game/HandTracking/SimonDice/BP_SimonLevel_Struct` (`|GetArrayItem` (`self.LevelSettings`) (`self.CurrentLevel`))))
  ; CreateRandomSequence Based On Level Settings
  (if (> (`KismetArrayLibrary.Array_Length` (`self.Stands`)) 0) :!label _label
    (if (> (`KismetArrayLibrary.Array_Length` (`self.PreviousSecuence`)) 0)
      (`KismetArrayLibrary.Array_Clear` (`self.SimonSequence`))
      (`KismetArrayLibrary.Array_Append` (`self.PreviousSecuence`) _simonsequence)
      (`KismetArrayLibrary.Array_Add` _simonsequence (`KismetMathLibrary.RandomIntegerInRange` 0 (`KismetArrayLibrary.Array_LastIndex` (`self.Stands`))))
      (`self.PlaySimonSequence`)
      (else
        (if _canduplicatenotes
          (`KismetArrayLibrary.Array_Add` (`self.SimonSequence`) (`KismetMathLibrary.RandomIntegerInRange` 0 (`KismetArrayLibrary.Array_LastIndex` (`self.Stands`))))
          (else
            (`KismetArrayLibrary.Array_AddUnique` (`self.SimonSequence`) (`KismetMathLibrary.RandomIntegerInRange` 0 (`KismetArrayLibrary.Array_LastIndex` (`self.Stands`))))))
        (if (< (`KismetArrayLibrary.Array_Length` (`self.SimonSequence`)) _numberofnotes)
          (`KismetSystemLibrary.Delay` 0.0)
          (goto _label)
          (else
            (`KismetSystemLibrary.Delay` 1.0)
            (`KismetArrayLibrary.Array_Clear` _previoussecuence)
            (`KismetArrayLibrary.Array_Append` (`self.SimonSequence`) _previoussecuence)
            (`self.PlaySimonSequence`)))))))

(event `self.ReceiveBeginPlay`
  (for _array_element (`self.Stands`)
    (`/Engine/EditorBlueprintResources/StandardMacros.IsValid` _array_element
      (:`Is Valid`
        (set `/Game/HandTracking/SimonDice/Bp_Stand.SimonMain_Ref` self _array_element))
      (:`Is Not Valid`
        (`KismetSystemLibrary.PrintString` "Forgot to SetUp Stands" true true (struct :`R` 1.0 :`G` 0.829394 :`A` 1.0) 5.0)))))

(event `ReallyStart`
  (if (not (`self.isPlaying`))
    (set `self.isPlaying` true)
    (for _array_element (`self.Stands`)
      (`/Game/HandTracking/SimonDice/Bp_Stand.DisableMoving` _array_element))
    (`self.StartLevel`)))

(event `StartLevel`
  (`KismetArrayLibrary.Array_Clear` (`self.PlayerSequence`))
  (set `self.CurrentNote` 0)
  (bind _output_get (set `self.isPlayersTurn` false))
  (set `self.Visible` _output_get)
  (`self.CreateSimonSequence`))

(event `PlaySimonSequence`
  (bind _textrender (`self.TextRender`))
  (bind _textrender_2 (`self.TextRender`))
  (`TextRenderComponent.K2_SetText` _textrender_2 (`self.Memoriza la secuencia`))
  (`TextRenderComponent.SetTextRenderColor` _textrender_2 (`self.TextColor_1`))
  (`/Game/HandTracking/SimonDice/Bp_Stand.PlayNote` (`|GetArrayItem` (`self.Stands`) (`|GetArrayItem` (`self.SimonSequence`) (`self.CurrentNote`))))
  (`KismetSystemLibrary.Delay` (`.TimeBetweenNotes_9_4C03084A4288E8E80A7167984C5690EA` (break `/Game/HandTracking/SimonDice/BP_SimonLevel_Struct` (`|GetArrayItem` (`self.LevelSettings`) (`self.CurrentLevel`)))))
  (`/Engine/EditorBlueprintResources/StandardMacros.IncrementInt` (`self.CurrentNote`)
    (:`  `
      (if (< (`self.CurrentNote`) (`KismetArrayLibrary.Array_Length` (`self.SimonSequence`)))
        (`self.PlaySimonSequence`)
        (else
          (bind _output_get (set `self.isPlayersTurn` true))
          (set `self.Visible` _output_get)
          (`TextRenderComponent.K2_SetText` _textrender (`self.TurnoJugador`))
          (`TextRenderComponent.SetTextRenderColor` _textrender (`self.TextColor_3`)))))))

(event `PlayerPlayedNote`
  (params (Note :type Integer))
  (set `self.isPlayersTurn` false)
  (bind _returnvalue (`KismetArrayLibrary.Array_Add` (`self.PlayerSequence`) Note))
  (if (== Note (`|GetArrayItem` (`self.SimonSequence`) _returnvalue))
    (`/Game/HandTracking/SimonDice/Bp_Stand.PlayNote` (`|GetArrayItem` (`self.Stands`) Note))
    (if (>= (`KismetArrayLibrary.Array_Length` (`self.PlayerSequence`)) (`KismetArrayLibrary.Array_Length` (`self.SimonSequence`)))
      (if (< (`self.CurrentLevel`) (`KismetArrayLibrary.Array_LastIndex` (`self.LevelSettings`)))
        (`/Engine/EditorBlueprintResources/StandardMacros.IncrementInt` (`self.CurrentLevel`)
          (:`  `
            (for _array_element (`self.Stands`)
              (`/Game/HandTracking/SimonDice/Bp_Stand.PlayComplete` _array_element)
              (`TextRenderComponent.K2_SetText` (`self.TextRender`) (`KismetTextLibrary.Conv_StringToText` (`KismetStringLibrary.Concat_StrStr` (`KismetTextLibrary.Conv_TextToString` (`self.Nivel actual`)) (`KismetStringLibrary.Conv_IntToString` (`self.CurrentLevel`))))))
            (bind _output_get (set `self.isPlayersTurn` false))
            (set `self.Visible` _output_get)
            (`KismetSystemLibrary.Delay` 1.0)
            (`self.StartLevel`)))
        (else
          (`GameplayStatics.PlaySound2D` "/Game/AuidosALMA/level-win-6416.level-win-6416" 1.0 1.0 0.0 null null)))
      (else
        (`KismetSystemLibrary.Delay` 0.5)
        (bind _output_get_2 (set `self.isPlayersTurn` true))
        (set `self.Visible` _output_get_2)))
    (else
      (for _array_element_2 (`self.Stands`)
        (`/Game/HandTracking/SimonDice/Bp_Stand.PlayError` _array_element_2))
      (`KismetSystemLibrary.Delay` 1.0)
      (`self.ReplaySecuence`))))

(event `ReplaySecuence`
  (bind _textrender (`self.TextRender`))
  (`KismetArrayLibrary.Array_Clear` (`self.PlayerSequence`))
  (set `self.CurrentNote` 0)
  (bind _output_get (set `self.isPlayersTurn` false))
  (set `self.Visible` _output_get)
  (`TextRenderComponent.K2_SetText` _textrender (`self.Memoriza la secuencia`))
  (`TextRenderComponent.SetTextRenderColor` _textrender (`self.TextColor_1`))
  (`/Game/HandTracking/SimonDice/Bp_Stand.PlayNote` (`|GetArrayItem` (`self.Stands`) (`|GetArrayItem` (`self.SimonSequence`) (`self.CurrentNote`))))
  (`KismetSystemLibrary.Delay` (`.TimeBetweenNotes_9_4C03084A4288E8E80A7167984C5690EA` (break `/Game/HandTracking/SimonDice/BP_SimonLevel_Struct` (`|GetArrayItem` (`self.LevelSettings`) (`self.CurrentLevel`)))))
  (`/Engine/EditorBlueprintResources/StandardMacros.IncrementInt` (`self.CurrentNote`)
    (:`  `
      (if (< (`self.CurrentNote`) (`KismetArrayLibrary.Array_Length` (`self.SimonSequence`)))
        (`self.PlaySimonSequence`)
        (else
          (bind _output_get_2 (set `self.isPlayersTurn` true))
          (set `self.Visible` _output_get_2)
          (`TextRenderComponent.K2_SetText` (`self.TextRender`) (`self.TurnoJugador`))
          (`TextRenderComponent.SetTextRenderColor` (`self.TextRender`) (`self.TextColor_3`)))))))

(event `self.ReceiveTick`
  (params (DeltaSeconds :type "Float (single-precision)"))
  (bind _returnvalue (`GameplayStatics.GetActorOfClass` "/Game/HandTracking/Blueprints/BP_HandsVR.BP_HandsVR_C"))
  (bind (_returnvalue_x _returnvalue_y _returnvalue_z) (`KismetMathLibrary.BreakVector` (`SceneComponent.K2_GetComponentLocation` (`/Game/HandTracking/Blueprints/BP_HandsVR.VR_Cam` _returnvalue))))
  (`self.K2_SetActorLocationAndRotation` (`KismetMathLibrary.MakeVector` (- _returnvalue_x 50.0) (+ _returnvalue_y 10.0) _returnvalue_z) (`KismetMathLibrary.MakeRotator` 0.0)))

(fn `UserConstructionScript`
  (bind _returnvalue (`KismetArrayLibrary.Array_Length` (`self.Stands`)))
  (for (_array_element _array_index) (`self.LevelSettings`)
    (bind (_numberofnotes _timebetweennotes _canduplicatenotes) (break `/Game/HandTracking/SimonDice/BP_SimonLevel_Struct` _array_element))
    (if _canduplicatenotes
      _
      (elif (> _numberofnotes _returnvalue)
        (bind _structout (setmembers `/Game/HandTracking/SimonDice/BP_SimonLevel_Struct` :`StructRef` _array_element :`NumberOfNotes` _returnvalue))
        (`KismetArrayLibrary.Array_Set` (`self.LevelSettings`) _array_index _structout)))))