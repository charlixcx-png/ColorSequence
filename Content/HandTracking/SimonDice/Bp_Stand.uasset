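; Colored pad for a hand-tracked VR Simon game that reports its index to SimonMainRef when touched during the player's turn.
; Note, error and completion events play sounds and briefly flash a dynamic material's intensity, the latter two also recoloring it.
; Tick looks up BP_Simon every frame, dimming the color while playing with Visible off.
; BeginPlay configures an Interaction SDK grab transformer, then immediately destroys the grabbable component.
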(event `self.ReceiveBeginPlay`
  (bind _isdkgrabtransformer (`self.IsdkGrabTransformer`))
  ; Activar Funcion Grab
  (bind _returnvalue (`|GenericCreateObject` "/Script/OculusInteraction.IsdkGrabFreeTransformer"))
  (`IsdkGrabTransformerComponent.SetSingleGrabTransformerObject` _isdkgrabtransformer _returnvalue)
  (set `IsdkGrabTransformerComponent.TransformTarget` (`self.StaticMesh`) _isdkgrabtransformer)
  (`self.DisableMoving`))

(event `self.StaticMesh.OnComponentBeginOverlap`
  (params (OverlappedComponent :type "PrimitiveComponent Object Reference") (OtherActor :type "Actor Object Reference") (OtherComp :type "PrimitiveComponent Object Reference") (OtherBodyIndex :type Integer) (bFromSweep :type Boolean) (SweepResult :type "HitResult Structure (by ref)"))
  (cast `/Game/HandTracking/Blueprints/BP_HandsVR` OtherActor)
  (bind _simonmain_ref (`self.SimonMain_Ref`)
    (:`then`
      (if (`/Game/HandTracking/SimonDice/BP_Simon.isPlayersTurn` _simonmain_ref)
        (`/Game/HandTracking/SimonDice/BP_Simon.PlayerPlayedNote` (`self.SimonMain_Ref`) (`self.Index`))))
    (:`else`)))

(event `PlayNote`
  (`GameplayStatics.PlaySoundAtLocation` (`self.PieceSound`) (0.0 0.0 0.0) (struct) 1.0 1.0 0.0 null null null null)
  (`MaterialInstanceDynamic.SetScalarParameterValue` (`self.DynMat`) "Intensity" 100.0)
  (`KismetSystemLibrary.Delay` 0.35)
  (`MaterialInstanceDynamic.SetScalarParameterValue` (`self.DynMat`) "Intensity" 0.0))

(event `PlayError`
  (`GameplayStatics.PlaySoundAtLocation` "/Engine/EditorSounds/Notifications/CompileFailed.CompileFailed" (0.0 0.0 0.0) (struct) 1.0 1.0 0.0 null null null null)
  (`MaterialInstanceDynamic.SetVectorParameterValue` (`self.DynMat`) "Color" (struct :`R` 1.0 :`A` 1.0))
  (`MaterialInstanceDynamic.SetScalarParameterValue` (`self.DynMat`) "Intensity" 100.0)
  (`KismetSystemLibrary.Delay` 0.35)
  (`MaterialInstanceDynamic.SetScalarParameterValue` (`self.DynMat`) "Intensity" 0.0)
  (`MaterialInstanceDynamic.SetVectorParameterValue` (`self.DynMat`) "Color" (`self.Color`)))

(event `PlayComplete`
  (`GameplayStatics.PlaySoundAtLocation` "/Engine/EditorSounds/Notifications/CompileSuccess_Cue.CompileSuccess_Cue" (0.0 0.0 0.0) (struct) 1.0 1.0 0.0 null null null null)
  (`MaterialInstanceDynamic.SetVectorParameterValue` (`self.DynMat`) "Color" (struct :`R` 0.252356 :`G` 1.0 :`A` 1.0))
  (`MaterialInstanceDynamic.SetScalarParameterValue` (`self.DynMat`) "Intensity" 100.0)
  (`KismetSystemLibrary.Delay` 0.35)
  (`MaterialInstanceDynamic.SetScalarParameterValue` (`self.DynMat`) "Intensity" 0.0)
  (`MaterialInstanceDynamic.SetVectorParameterValue` (`self.DynMat`) "Color" (`self.Color`)))

(event `self.ReceiveTick`
  (params (DeltaSeconds :type "Float (single-precision)"))
  (bind _returnvalue (`GameplayStatics.GetActorOfClass` "/Game/HandTracking/SimonDice/BP_Simon.BP_Simon_C"))
  (if (`/Game/HandTracking/SimonDice/BP_Simon.isPlaying` _returnvalue)
    (if (`/Game/HandTracking/SimonDice/BP_Simon.Visible` _returnvalue)
      (`MaterialInstanceDynamic.SetVectorParameterValue` (`self.DynMat`) "Color" (`self.Color`))
      (else
        (`MaterialInstanceDynamic.SetVectorParameterValue` (`self.DynMat`) "Color" (* (`self.Color`) (struct :`R` 0.135417 :`G` 0.135417 :`B` 0.135417 :`A` 1.0)))))))

(fn `DisableMoving`
  (bind _isdkgrabbable (`self.IsdkGrabbable`))
  (`ActorComponent.SetActive` _isdkgrabbable false false)
  (`ActorComponent.K2_DestroyComponent` _isdkgrabbable))

(fn `UserConstructionScript`
  (bind _returnvalue (`PrimitiveComponent.CreateDynamicMaterialInstance` (`self.StaticMesh`) 0 "/Game/HandTracking/Blueprints/M_Color.M_Color" "None"))
  (bind _output_get (set `self.DynMat` _returnvalue))
  (`MaterialInstanceDynamic.SetVectorParameterValue` _output_get "Color" (`self.Color`)))