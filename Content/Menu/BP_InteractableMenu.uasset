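; BP_InteractableMenu is a VR menu actor that opens a level after repeated contact from the player's BP_HandsVR.
; Every Tick it looks up BP_HandsVR and places itself at a fixed world-X offset from its camera, with a fixed rotation.
; Mesh collision is disabled for a few seconds after BeginPlay, then becomes query-only.
; Mesh overlaps with BP_HandsVR increment a counter, and once it hits the threshold the next overlap opens the Sequence level.
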(event `self.ReceiveBeginPlay`
  (`PrimitiveComponent.SetCollisionEnabled` (`self.StaticMesh`) "NoCollision")
  (`KismetSystemLibrary.Delay` 3.0)
  (`PrimitiveComponent.SetCollisionEnabled` (`self.StaticMesh`) "QueryOnly"))

(event `self.ReceiveTick`
  (params (DeltaSeconds :type "Float (single-precision)"))
  (bind _returnvalue (`GameplayStatics.GetActorOfClass` "/Game/HandTracking/Blueprints/BP_HandsVR.BP_HandsVR_C"))
  (bind (_returnvalue_x _returnvalue_y _returnvalue_z) (`KismetMathLibrary.BreakVector` (`SceneComponent.K2_GetComponentLocation` (`/Game/HandTracking/Blueprints/BP_HandsVR.VR_Cam` _returnvalue))))
  (`self.K2_SetActorLocationAndRotation` (`KismetMathLibrary.MakeVector` (+ _returnvalue_x 50.0) _returnvalue_y _returnvalue_z) (struct :`Yaw` -180.0)))

(event `self.StaticMesh.OnComponentBeginOverlap`
  (params (OverlappedComponent :type "PrimitiveComponent Object Reference") (OtherActor :type "Actor Object Reference") (OtherComp :type "PrimitiveComponent Object Reference") (OtherBodyIndex :type Integer) (bFromSweep :type Boolean) (SweepResult :type "HitResult Structure (by ref)"))
  (cast `/Game/HandTracking/Blueprints/BP_HandsVR` OtherActor)
  (if (>= (`self.NumOverlaps`) 5)
    (`GameplayStatics.OpenLevelBySoftObjectPtr` "/Game/VRTemplate/Maps/Sequence.Sequence")
    (else
      (`/Engine/EditorBlueprintResources/StandardMacros.IncrementInt` (`self.NumOverlaps`)))))

(fn `UserConstructionScript`)