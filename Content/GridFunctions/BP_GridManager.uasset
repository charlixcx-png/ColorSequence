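; BP_GridManager arranges Bp_Stand actors into a 3D grid as they enter its Area.
; BeginPlay fills Posisiones with a cubic lattice of offsets spaced by Separacion.
; Each overlapping stand is swept to the relative location indexed by NumStands, then attached to Area keeping relative transforms.
; The counter then advances with no bounds check, and a debug string prints on each placement.
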(event `self.ReceiveBeginPlay`
  (`KismetArrayLibrary.Array_Clear` (`self.Posisiones`))
  (for _index (range 4)
    (for _index_2 (range 4)
      (for _index_3 (range 4)
        (`KismetArrayLibrary.Array_Add` (`self.Posisiones`) (`KismetMathLibrary.MakeVector` (* _index (`self.Separacion`)) (* _index_2 (`self.Separacion`)) (* _index_3 (`self.Separacion`))))))))

(event `self.Area.OnComponentBeginOverlap`
  (params (OverlappedComponent :type "PrimitiveComponent Object Reference") (OtherActor :type "Actor Object Reference") (OtherComp :type "PrimitiveComponent Object Reference") (OtherBodyIndex :type Integer) (bFromSweep :type Boolean) (SweepResult :type "HitResult Structure (by ref)"))
  (bind _asbp_stand (cast `/Game/HandTracking/SimonDice/Bp_Stand` OtherActor))
  (`self.Agregar objeto al grid` _asbp_stand)
  (`KismetSystemLibrary.PrintString` "aaaaaaaaaa")
  (`self.K2_AttachToComponent` _asbp_stand (`self.Area`) "None" "KeepRelative" "KeepRelative" "KeepRelative" false)
  (`/Engine/EditorBlueprintResources/StandardMacros.IncrementInt` (`self.NumStands`)))

(fn `Agregar objeto al grid`
  (params (Actor :type "/Game/HandTracking/SimonDice/Bp_Stand Object Reference"))
  (`self.K2_SetActorRelativeLocation` Actor (`|GetArrayItem` (`self.Posisiones`) (`self.NumStands`)) true false))

(fn `UserConstructionScript`)