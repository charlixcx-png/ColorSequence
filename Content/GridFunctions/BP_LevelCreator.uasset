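; VR level-setup actor that arranges the level's Bp_Stand actors in a grid on a grabbable root.
; On BeginPlay, for each "Start"-tagged widget, it attaches the widget, moves itself near the BP_HandsVR camera and computes a near-square grid from TotalObjetos.
; It then moves existing stands into those slots and attaches them; the stand-spawning branch is unused.
; DisableMoving destroys the grabbable component to stop movement.
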(event `self.ReceiveBeginPlay`
  (bind _cols (`self.Cols`))
  (bind (_relativelocation_x _relativelocation_y _relativelocation_z) (`KismetMathLibrary.BreakVector` (`SceneComponent.RelativeLocation` (`self.Cube`))))
  (bind _outactors (`GameplayStatics.GetAllActorsOfClassWithTag` "/Script/OculusInteractionPrebuilts.IsdkInteractableWidget" "Start"))
  (for _array_element _outactors
    (`self.K2_AttachToComponent` _array_element (`self.DefaultSceneRoot`) "None" "KeepRelative" "KeepRelative" "KeepWorld" true)
    (bind _returnvalue (`GameplayStatics.GetActorOfClass` "/Game/HandTracking/Blueprints/BP_HandsVR.BP_HandsVR_C"))
    (bind (_returnvalue_x _returnvalue_y _returnvalue_z) (`KismetMathLibrary.BreakVector` (`SceneComponent.K2_GetComponentLocation` (`/Game/HandTracking/Blueprints/BP_HandsVR.VR_Cam` _returnvalue))))
    (`self.K2_SetActorLocation` (`KismetMathLibrary.MakeVector` (- _returnvalue_x 60.0) _returnvalue_y (+ _returnvalue_z 100.0)))
    (`KismetArrayLibrary.Array_Clear` (`self.PosicionesPred`))
    (set `self.Cols` (`KismetMathLibrary.FCeil` (`KismetMathLibrary.Sqrt` (`KismetMathLibrary.Conv_IntToDouble` (`self.TotalObjetos`)))))
    (set `self.Rows` (/ (`self.TotalObjetos`) (`self.Cols`)))
    (for _index (range (`self.TotalObjetos`))
      (`KismetArrayLibrary.Array_Add` (`self.PosicionesPred`) (`KismetMathLibrary.MakeVector` _relativelocation_x (+ (- _relativelocation_y (* (- (`self.Cols`) 1) (/ (`self.EspacioEntreObj`) 2.0))) (* (mod _index _cols) (`self.EspacioEntreObj`))) (- (+ (- 0.0 _relativelocation_z) (* (/ _index _cols) (`self.EspacioEntreObj`))) (/ (`self.EspacioEntreObj`) 1.3)))))
    (bind _outactors_2 (`GameplayStatics.GetAllActorsOfClass` "/Game/HandTracking/SimonDice/Bp_Stand.Bp_Stand_C"))
    (for (_array_element_2 _array_index) _outactors_2
      (`self.K2_SetActorLocation` _array_element_2 (`|GetArrayItem` (`self.PosicionesPred`) _array_index) true false)
      (`self.K2_AttachToComponent` _array_element_2 (`self.DefaultSceneRoot`) "None" "KeepRelative" "KeepRelative" "KeepWorld" true))))

(fn `DisableMoving`
  (bind _isdkgrabbable (`self.IsdkGrabbable`))
  (`ActorComponent.SetActive` _isdkgrabbable false false)
  (`ActorComponent.K2_DestroyComponent` _isdkgrabbable))

(fn `NewFunction`
  (returns (ReturnValue :type "Actor Object Reference"))
  (return null))

(fn `UserConstructionScript`)